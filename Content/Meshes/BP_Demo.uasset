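; BP_Demo builds a flat X/Y grid of instanced static meshes at BeginPlay and spawns a BP_DemoTest actor on each instance.
; Nested loops add instances spaced by GridSize on a component scaled by GridScale, recording their indices in GridIndex.
; A second pass spawns the actors, owned by this Blueprint, at each instance's world-space transform.
; GridLocation is cleared at the start but never filled here.
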(event EventBeginPlay
  (bind _gridsize (Variables|Default|GetGridSize))
  (Utilities|FlowControl|Sequence
    (:then_0
      (Transformation|SetWorldScale3D (Variables|Default|GetInstancedStaticMesh) (Variables|Default|GetGridScale))
      (Utilities|Array|Clear (Variables|Default|GetGridLocation))
      (for _index (range 0 (- (Variables|Default|GetGridX) 1))
        (for _index_2 (range 0 (- (Variables|Default|GetGridY) 1))
          (bind _returnvalue (Components|InstancedStaticMesh|AddInstance (Variables|Default|GetInstancedStaticMesh) (Math|Transform|MakeTransform (Math|Vector|MakeVector (* _index _gridsize) (* _index_2 _gridsize) 0.0))))
          (Utilities|Array|Add (Variables|Default|GetGridIndex) _returnvalue))))
    (:then_1
      (for _array_element (Variables|Default|GetGridIndex)
        (Game|SpawnActorfromClass "/Game/Meshes/BP_DemoTest.BP_DemoTest_C" (.OutInstanceTransform (Components|InstancedStaticMesh|GetInstanceTransform (Variables|Default|GetInstancedStaticMesh) _array_element true)) "Undefined" self 0)))))

(fn ConstructionScript)