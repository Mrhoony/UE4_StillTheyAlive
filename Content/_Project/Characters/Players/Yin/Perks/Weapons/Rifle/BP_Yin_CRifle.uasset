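; Rifle weapon actor for the player character Yin, handling how the rifle appears when equipped and unequipped.
; On BeginPlay it attaches to the Hand_Rifle socket, then hides its skeletal mesh if the owner is a CPlayer.
; The equip event shows the mesh and reattaches it to that socket, while unequip only hides it, without detaching.
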(event EventBeginPlay
  (Class|CAttachment|Attachto "Hand_Rifle")
  (Utilities|Casting|CastToCPlayer (Components|GetOwner))
  (Rendering|SetVisibility (Variables|Default|GetSkeletalMesh) false false))

(event Collision|EventActorBeginOverlap
  (params (OtherActor :type Actor%20Object%20Reference)))

(event EventTick
  (params (DeltaSeconds :type Float%20%28single-precision%29)))

(event EventOnEquip
  (Rendering|SetVisibility (Variables|Default|GetSkeletalMesh) true false)
  (Class|CAttachment|Attachto "Hand_Rifle"))

(event EventOnUnequip
  (Rendering|SetVisibility (Variables|Default|GetSkeletalMesh) false false))

(fn ConstructionScript)